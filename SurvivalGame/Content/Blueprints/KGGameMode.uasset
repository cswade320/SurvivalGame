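; KGGameMode is a game mode that runs wave-based enemy spawning and handles game win and death endings.
; Each wave's class list is shuffled into a queue, which a looping one-second timer drains by spawning AI at random PlayerStarts.
; Destroy events trigger the next wave once the queue and AI controllers are gone; exhausting waves means victory.
; Both endings fire a dispatcher, blend to a camera actor, then show their screen after a delay.
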(event Custom|SpawnEnemy
  (if (> (Utilities|Array|Length (Variables|Default|GetCurrentQueue)) 0)
    (bind _outactors (Actor|GetAllActorsOfClass "/Script/Engine.PlayerStart"))
    (bind _returnvalue (AI|SpawnAIFromClass (Utilities|Array|Get(acopy) (Variables|Default|GetCurrentQueue)) 0 (Transformation|GetActorLocation (Utilities|Array|Get(acopy) _outactors (Math|Random|RandomInteger (Utilities|Array|Length _outactors)))) (Transformation|GetActorRotation (Utilities|Array|Get(acopy) _outactors (Math|Random|RandomInteger (Utilities|Array|Length _outactors)))) false))
    (Utilities|Array|RemoveIndex (Variables|Default|GetCurrentQueue))
    (Game|BindEventtoOnDestroyed _returnvalue (delegate Custom|CheckWaveComplete))))

(event Custom|StartNewWave
  (Math|Integer|IncrementInt (Variables|Default|GetWaveIndex)
    (:%20%20
      (Default|CallNewWave)
      (if (< (Utilities|Array|LastIndex (Variables|Default|GetWaves)) (Variables|Default|GetWaveIndex))
        (CallFunction|EndGameWin)
        (else
          (bind _output_get (Variables|Default|SetCurrentQueue (.classtospawn (Utilities|Array|Get(acopy) (Variables|Default|GetWaves) (Variables|Default|GetWaveIndex)))))
          (Utilities|Array|Shuffle _output_get))))))

(event Custom|EndGameDeath
  (bind _returnvalue (Game|GetPlayerController 0))
  (Default|CallEndGameDispatch)
  (bind _outactors (Actor|GetAllActorsOfClass "/Script/Engine.CameraActor"))
  (Game|Player|SetViewTargetwithBlend _returnvalue (Utilities|Array|Get(acopy) _outactors) 4.0 "VTBlend_Linear" 0.0 true)
  (Utilities|FlowControl|Delay 6.0)
  (bind _askgplayer_controller_base (Utilities|Casting|CastToKGPlayerControllerBase _returnvalue))
  (Variables|Default|SetPlayerControllerBaseReference _askgplayer_controller_base)
  (UserInterface|Viewport|AddtoViewport (Variables|/Game/Blueprints/KGPlayerControllerBase.KGPlayerControllerBase_C|GetGameOverSreenReference (Variables|Default|GetPlayerControllerBaseReference)) 0))

(event Custom|CheckWaveComplete
  (params (DestroyedActor :type Actor%20Object%20Reference))
  (if (== (Utilities|Array|Length (Variables|Default|GetCurrentQueue)) 0)
    (bind _outactors (Actor|GetAllActorsOfClass "/Game/Blueprints/KGAIControllerBase.KGAIControllerBase_C"))
    (if (== (Utilities|Array|Length _outactors) 0)
      (CallFunction|StartNewWave))))

(event Custom|ResetGame
  (Variables|Default|SetWaveIndex 0)
  (bind _output_get (Variables|Default|SetCurrentQueue (.classtospawn (Utilities|Array|Get(acopy) (Variables|Default|GetWaves) (Variables|Default|GetWaveIndex)))))
  (Utilities|Array|Shuffle _output_get))

(event Custom|EndGameWin
  (bind _returnvalue (Game|GetPlayerController 0))
  (Default|CallEndGameDispatch)
  (bind _outactors (Actor|GetAllActorsOfClass "/Script/Engine.CameraActor"))
  (Game|Player|SetViewTargetwithBlend _returnvalue (Utilities|Array|Get(acopy) _outactors) 4.0 "VTBlend_Linear" 0.0 true)
  (Utilities|FlowControl|Delay 6.0)
  (bind _askgplayer_controller_base (Utilities|Casting|CastToKGPlayerControllerBase _returnvalue))
  (Variables|Default|SetPlayerControllerBaseReference _askgplayer_controller_base)
  (UserInterface|Viewport|AddtoViewport (Variables|/Game/Blueprints/KGPlayerControllerBase.KGPlayerControllerBase_C|GetGameWinScreenReference (Variables|Default|GetPlayerControllerBaseReference)) 0))

(event EventBeginPlay
  (Utilities|Time|SetTimerbyEvent (delegate Custom|SpawnEnemy) 1.0 true)
  (CallFunction|REsetGame))

(event EventTick
  (params (DeltaSeconds :type Float%20%28single-precision%29)))

(fn ConstructionScript)